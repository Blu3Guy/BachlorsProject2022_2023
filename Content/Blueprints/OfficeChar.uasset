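; First-person player character with walk, run, crouch, flashlight, right-mouse zoom, pause menu and look-at inspection.
; Timelines drive zoom FOV and crouch capsule height with post-processing; forward-axis input picks idle, walk or run camera shakes from velocity.
; Tick sets walk speed and line-traces from the camera, using InspectInterface on physics-simulating hits to toggle custom depth and HUD messages.
; PickUp and Drop are empty stubs.
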(event EventBeginPlay
  (bind _returnvalue (UserInterface|CreateWidget "/Game/Blueprints/Interface/HeadsUpDisplay.HeadsUpDisplay_C"))
  (bind _output_get (Variables|Default|SetHeadsUpDisplay _returnvalue))
  (UserInterface|Viewport|AddtoViewport _output_get 0)
  (bind _returnvalue_2 (UserInterface|CreateWidget "/Game/Blueprints/HUD/HUD.HUD_C"))
  (UserInterface|Viewport|AddtoViewport _returnvalue_2 0)
  (Variables|Default|SetbIsRunning false)
  (Variables|Default|SetRunSpeed 3.5e+02)
  (Utilities|FlowControl|Sequence
    (:then_0
      (Variables|Default|SetDefaultCameraLocation (Variables|/Script/Engine.SceneComponent|GetRelativeLocation (Variables|Default|GetFirstPersonCamera))))))

(event EventTick
  (params (DeltaSeconds :type Float%20%28single-precision%29))
  (bind _charactermovement (Variables|Character|GetCharacterMovement))
  (bind _charactermovement_2 (Variables|Character|GetCharacterMovement))
  (CallFunction|InteractTrace 5e+02)
  (Utilities|FlowControl|Sequence
    (:then_0
      ;[1 1 1] Crouch
      (if (Variables|Default|GetIsCrouched)
        (Variables|/Script/Engine.CharacterMovementComponent|SetMaxWalkSpeed _charactermovement_2 (Variables|Default|GetWalkSpeed))
        (else
          (Variables|/Script/Engine.CharacterMovementComponent|SetMaxWalkSpeed _charactermovement_2 (Variables|Default|GetCrouchSpeed))))
      (if (Variables|Default|GetbIsRunning)
        (if (Variables|Default|GetIsCrouched)
          (Variables|/Script/Engine.CharacterMovementComponent|SetMaxWalkSpeed _charactermovement (Variables|Default|GetRunSpeed)))
        (else
          (Variables|/Script/Engine.CharacterMovementComponent|SetMaxWalkSpeed _charactermovement (Variables|Default|GetWalkSpeed)))))))

(event Input|ActionEvents|InputActionPause
  (params (Key :type Key%20Structure :default "None"))
  (bind _returnvalue (Game|GetPlayerController 0))
  ;[1 1 1] Pause/Un-pause Game
  (:Pressed
    (Utilities|IsValid (Variables|Default|GetPause%20Menu%20REF)
      (:Is%20Valid
        _)
      (:Is%20Not%20Valid
        (bind _returnvalue_2 (UserInterface|CreateWidget "/Game/Blueprints/UI/Pause_Menu/Pause_Menu.Pause_Menu_C"))
        (Variables|Default|SetPause%20Menu%20REF _returnvalue_2)))
    (if (Game|IsGamePaused)
      (Widget|RemovefromParent (Variables|Default|GetPause%20Menu%20REF))
      (Game|SetGamePaused false)
      (Variables|/Script/Engine.PlayerController|SetbShowMouseCursor _returnvalue false)
      (Input|SetInputModeGameOnly _returnvalue false)
      (else
        (UserInterface|Viewport|AddtoViewport (Variables|Default|GetPause%20Menu%20REF) 0)
        (Game|SetGamePaused true)
        (Variables|/Script/Engine.PlayerController|SetbShowMouseCursor _returnvalue true)
        (Input|SetInputModeUIOnly _returnvalue (Variables|Default|GetPause%20Menu%20REF) "LockInFullscreen" false)))))

(event Input|ActionEvents|InputActionFlashlight
  (params (Key :type Key%20Structure :default "None"))
  ;[1 1 1] Flashlight
  (:Pressed
    (Rendering|SetVisibility (Variables|Default|GetFlashlight) (not (Rendering|IsVisible (Variables|Default|GetFlashlight))) false)))

(event Input|AxisEvents|InputAxisForwards/Backwards
  (params (AxisValue :type Float%20%28single-precision%29))
  (bind _returnvalue (Transformation|GetVelocity))
  (bind _returnvalue_2 (Transformation|GetActorLocation))
  (bind _returnvalue_3 (Math|Vector|VectorLength _returnvalue))
  ;[1 1 1] Basic Movement
  (Pawn|Input|AddMovementInput (Math|Vector|GetForwardVector (Math|Rotator|MakeRotator 0.0 0.0 (.Yaw (Math|Rotator|BreakRotator (Pawn|GetControlRotation :!class /Script/Engine.Pawn))))) AxisValue false)
  (if (<= _returnvalue_3 1.0)
    (Camera|PlayWorldCameraShake "/Game/Blueprints/IdleShake.IdleShake_C" _returnvalue_2 1e+02 0.0)
    (elif (>= _returnvalue_3 349.0)
      (Camera|PlayWorldCameraShake "/Game/Blueprints/RunShake.RunShake_C" _returnvalue_2 1e+02 0.0)
      (else
        (Camera|PlayWorldCameraShake "/Game/Blueprints/WalkShake.WalkShake_C" _returnvalue_2 1e+02 0.0)))))

(event Input|AxisEvents|InputAxisRight/Left
  (params (AxisValue :type Float%20%28single-precision%29))
  ;[1 1 1] Basic Movement
  (Pawn|Input|AddMovementInput (Math|Vector|GetRightVector (Math|Rotator|MakeRotator 0.0 0.0 (.Yaw (Math|Rotator|BreakRotator (Pawn|GetControlRotation :!class /Script/Engine.Pawn))))) AxisValue false))

(event Input|AxisEvents|InputAxisViewUpDown
  (params (AxisValue :type Float%20%28single-precision%29))
  ;[1 1 1] Basic Camera Movement
  (Pawn|Input|AddControllerPitchInput AxisValue))

(event Input|AxisEvents|InputAxisviewLeftRight
  (params (AxisValue :type Float%20%28single-precision%29))
  ;[1 1 1] Basic Camera Movement
  (Pawn|Input|AddControllerYawInput AxisValue))

(event Input|KeyboardEvents|LeftShift
  (params (Key :type Key%20Structure :default "None"))
  (:Pressed
    (Variables|Default|SetbIsRunning true))
  (:Released
    (Variables|Default|SetbIsRunning false)))

(event Input|KeyboardEvents|LeftCtrl
  (params (Key :type Key%20Structure :default "None"))
  ;[1 1 1] Crouch
  (:Pressed
    (Variables|Default|SetIsCrouched false)
    (bind _offsetvalue (Timeline|Crouch%20Height PlayFromStart)
      (:Update
        (Components|Capsule|SetCapsuleHalfHeight (Variables|Collision|GetCapsuleComponent) (- 96.0 (* _offsetvalue (Variables|Default|GetHalfHeightOffset))) true)
        (Variables|/Script/Engine.CameraComponent|SetPostProcessSettings (Variables|Default|GetFirstPersonCamera) (Utilities|Struct|MakePostProcessSettings (* _offsetvalue 0.7))))))
  (:Released
    (Variables|Default|SetIsCrouched true)
    (Timeline|Crouch%20Height ReverseFromEnd)))

(event Input|MouseEvents|RightMouseButton
  (params (Key :type Key%20Structure :default "None"))
  ;[1 1 1] zoom
  (:Pressed
    (bind _zoom (Timeline|Zoom Play)
      (:Update
        (Camera|SetFieldOfView (Variables|Default|GetFirstPersonCamera) _zoom))))
  (:Released
    (Timeline|Zoom Reverse)))

(fn ConstructionScript)

(fn PickUp)

(fn Drop)

(fn InteractTrace
  (params (Range :type Float%20%28double-precision%29))
  (bind _firstpersoncamera (Variables|Default|GetFirstPersonCamera))
  (bind _returnvalue (Transformation|GetWorldLocation _firstpersoncamera))
  ;[1 1 1] TraceChannel.
  (bind _outhit (Collision|LineTraceByChannel _returnvalue (+ _returnvalue (* (Math|Vector|GetForwardVector _firstpersoncamera) (Math|Conversions|ToVector(Float) Range))) "TraceTypeQuery1" false 0 "None"))
  (if true
    (LocalVariables|SetLoc_HitResults _outhit)
    (if (!= (Variables|Default|GetLookAtComponent) (.HitComponent (Collision|BreakHitResult _outhit)))
      (bind _lookatcomponent (Variables|Default|GetLookAtComponent)
        (:then
          (Rendering|SetRenderCustomDepth _lookatcomponent true))
        (:else
          _))
      (if (and (Utilities|DoesObjectImplementInterface (.HitActor (Collision|BreakHitResult _outhit)) "/Game/Blueprints/Interface/InspectInterface.InspectInterface_C") (Physics|IsSimulatingPhysics (.HitComponent (Collision|BreakHitResult _outhit)) "None"))
        (bind (_lookatactor _lookatcomponent_2 _message) (Class|InspectInterface|Lookat(Message) (.HitActor (Collision|BreakHitResult (LocalVariables|GetLoc_HitResults))) self (Game|GetPlayerController 0) (.HitComponent (Collision|BreakHitResult (LocalVariables|GetLoc_HitResults)))))
        (bind _output_get (Variables|Default|SetLookAtComponent _lookatcomponent_2))
        (Rendering|SetRenderCustomDepth _output_get true)
        (Default|DisplayMessage (Variables|Default|GetHeadsUpDisplay) _message)
        (else
          (bind _lookatcomponent_3 (Variables|Default|GetLookAtComponent)
            (:then
              (Rendering|SetRenderCustomDepth _lookatcomponent_3 false)
              (Variables|Default|SetLookAtComponent 0)
              (Default|DisplayMessage (Variables|Default|GetHeadsUpDisplay)))
            (:else))))
      (else
        (bind _lookatcomponent_4 (Variables|Default|GetLookAtComponent)
          (:then
            (Rendering|SetRenderCustomDepth _lookatcomponent_4 false)
            (Variables|Default|SetLookAtComponent 0)
            (Default|DisplayMessage (Variables|Default|GetHeadsUpDisplay)))
          (:else))))))