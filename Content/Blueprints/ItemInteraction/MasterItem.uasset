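; Base actor for inspectable items, showing an interact indicator while the OfficeChar overlaps its sphere.
; InspectInteract_1 disables collision, attaches the item to the camera manager, zooms it, opens an InspectUI with name and description, and moves input from player to item.
; While inspecting, left-mouse drag or movement axes rotate the item.
; Interact detaches it, returns it to its BeginPlay transform, and restores collision and player input.
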(event OnComponentBeginOverlap(Sphere)
  (params (OverlappedComponent :type Primitive%20Component%20Object%20Reference) (OtherActor :type Actor%20Object%20Reference) (OtherComp :type Primitive%20Component%20Object%20Reference) (OtherBodyIndex :type Integer) (bFromSweep :type Boolean) (SweepResult :type Hit%20Result%20Structure%20%28by%20ref%29))
  (Utilities|Casting|CastToOfficeChar OtherActor)
  (Rendering|SetVisibility (Variables|Default|GetInteractIndicator) true false))

(event OnComponentEndOverlap(Sphere)
  (params (OverlappedComponent :type Primitive%20Component%20Object%20Reference) (OtherActor :type Actor%20Object%20Reference) (OtherComp :type Primitive%20Component%20Object%20Reference) (OtherBodyIndex :type Integer))
  (Utilities|Casting|CastToOfficeChar OtherActor)
  (Rendering|SetVisibility (Variables|Default|GetInteractIndicator) false false))

(event Custom|InspectInteract_1
  (params (Player :type Office%20Char%20Object%20Reference))
  (bind _returnvalue (Game|GetPlayerController 0))
  (Variables|Default|SetPlayer Player)
  (Collision|SetActorEnableCollision false)
  (Collision|SetCollisionProfileName (Variables|Default|GetSphere) "NoCollision" true :!class /Script/Engine.PrimitiveComponent)
  (Transformation|AttachComponentToComponent (Variables|/Script/Engine.PlayerCameraManager|GetTransformComponent (Game|GetPlayerCameraManager 0)) "None" "KeepWorld" "KeepWorld" "KeepWorld" true)
  (bind _returnvalue_2 (Game|ConstructObjectfromClass "/Game/Blueprints/ItemInteraction/InspectUI.InspectUI_C" (Variables|Default|GetItemName) (Variables|Default|GetItemDescription)))
  (bind _output_get (Variables|Default|SetIspectUI _returnvalue_2))
  (UserInterface|Viewport|AddtoViewport _output_get 0)
  (Components|MoveComponentTo (Variables|Default|GetDefaultSceneRoot) (Math|Vector|MakeVector (Variables|Default|GetZoomAmount) 0.0 0.0) "0, 0, 0" false false 0.2 false)
  (Input|DisableInput (Variables|Default|GetPlayer) _returnvalue)
  (Input|EnableInput _returnvalue))

(event EventBeginPlay
  (Variables|Default|SetNewVar (Transformation|GetActorTransform)))

(event Input|ActionEvents|InputActionInteract
  (params (Key :type Key%20Structure))
  (bind _returnvalue (Game|GetPlayerController 0))
  (bind _newvar (Variables|Default|GetNewVar))
  (:Pressed
    (Transformation|DetachFromActor "KeepWorld" "KeepWorld" "KeepWorld")
    (Widget|RemovefromParent (Variables|Default|GetIspectUI))
    (Variables|Default|SetIspectUI 0)
    (Components|MoveComponentTo (Variables|Default|GetDefaultSceneRoot) (.location _newvar) (.rotation _newvar) false false 0.2 false)
    (Collision|SetActorEnableCollision true)
    (Collision|SetCollisionProfileName (Variables|Default|GetSphere) "OverlapAllDynamic" true :!class /Script/Engine.PrimitiveComponent)
    (Input|DisableInput _returnvalue)
    (Input|EnableInput (Variables|Default|GetPlayer) _returnvalue)))

(event Input|AxisEvents|InputAxisForwards/Backwards
  (params (AxisValue :type Float%20%28single-precision%29))
  (if (!= AxisValue 0.0)
    (Transformation|SetActorRotation (Math|Rotator|CombineRotators (Transformation|GetActorRotation) (Math|Rotator|MakeRotator (* AxisValue 1.0) 0.0 0.0)))))

(event Input|AxisEvents|InputAxisRight/Left
  (params (AxisValue :type Float%20%28single-precision%29))
  (if (!= AxisValue 0.0)
    (Transformation|SetActorRotation (Math|Rotator|CombineRotators (Transformation|GetActorRotation) (Math|Rotator|MakeRotator 0.0 0.0 (* AxisValue 1.0))))))

(event Input|MouseEvents|MouseX
  (params (AxisValue :type Float%20%28single-precision%29))
  (if (Variables|Default|GetCanRotate)
    (Transformation|SetActorRotation (Math|Rotator|CombineRotators (Transformation|GetActorRotation) (Math|Rotator|MakeRotator 0.0 0.0 (* AxisValue -2.0))))))

(event Input|MouseEvents|MouseY
  (params (AxisValue :type Float%20%28single-precision%29))
  (if (Variables|Default|GetCanRotate)
    (Transformation|SetActorRotation (Math|Rotator|CombineRotators (Transformation|GetActorRotation) (Math|Rotator|MakeRotator (* AxisValue -2.0) 0.0 0.0)))))

(event Input|MouseEvents|LeftMouseButton
  (params (Key :type Key%20Structure))
  (:Pressed
    (Variables|Default|SetCanRotate true))
  (:Released
    (Variables|Default|SetCanRotate false)))

(fn ConstructionScript)