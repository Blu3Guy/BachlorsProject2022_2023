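; Door for the ruined research room that swings open on an inspect interaction and has no close logic.
; BeginPlay stores the starting yaw and sets an absolute end yaw, and the interaction sets a Rotate flag that is never cleared.
; Tick calls PlayFromStart or ReverseFromEnd every frame based on that flag, restarting the Timeline whose update lerps the actor's yaw between the two angles.
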(event EventTick
  (params (DeltaSeconds :type Float%20%28single-precision%29))
  (if (stale EventInspectInteract1 _output_get)
    (bind _newtrack_0 (Timeline|Timeline PlayFromStart)
      (:Update
        (Transformation|SetActorRotation (Math|Rotator|MakeRotator 0.0 0.0 (Math|Float|Lerp (Variables|Default|GetStartRotation) (Variables|Default|GetEndRotation) _newtrack_0)))))
    (else
      (Timeline|Timeline ReverseFromEnd))))

(event EventInspectInteract1
  (params (Player :type Office%20Char%20Object%20Reference))
  (bind _output_get (Variables|Default|SetbRotate true)))

(event EventBeginPlay
  (Variables|Default|SetStartRotation (.yaw (Transformation|GetActorRotation)))
  (Variables|Default|SetEndRotation 9e+01))

(fn ConstructionScript
  (|CallParentFunction))