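; Research room door that, when interacted with, swings open and transitions the player to the Facility level.
; InspectInteract1 sets a Rotate flag that Tick polls to lock input to UI-only and play a timeline.
; The timeline lerps yaw from the starting rotation to a fixed angle.
; Its Update output also drives the delayed chain that shows a loading screen, then opens the level.
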(event EventTick
  (params (DeltaSeconds :type Float%20%28single-precision%29))
  (if (stale EventInspectInteract1 _output_get)
    (Input|SetInputModeUIOnly (Game|GetPlayerController 0) 0 "LockAlways" false)
    (bind _newtrack_0 (Timeline|Timeline Play)
      (:Update
        (Transformation|SetActorRotation (Math|Rotator|MakeRotator 0.0 0.0 (Math|Float|Lerp (Variables|Default|GetStartRotation) (Variables|Default|GetEndRotation) _newtrack_0)))
        (Utilities|FlowControl|Delay 3.0)
        (bind _returnvalue (UserInterface|CreateWidget "/Game/Blueprints/UI/LoadingScreen.LoadingScreen_C" (Game|GetPlayerController 0)))
        (UserInterface|Viewport|AddtoViewport _returnvalue 0)
        (Utilities|FlowControl|Delay 5.0)
        (Game|OpenLevel(byName) "Facility")))))

(event EventInspectInteract1
  (params (Player :type Office%20Char%20Object%20Reference))
  (bind _output_get (Variables|Default|SetbRotate true)))

(event EventBeginPlay
  (Variables|Default|SetStartRotation (.yaw (Transformation|GetActorRotation)))
  (Variables|Default|SetEndRotation 2e+01))

(fn ConstructionScript
  (|CallParentFunction))