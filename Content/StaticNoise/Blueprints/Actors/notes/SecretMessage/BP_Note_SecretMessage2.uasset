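; BP_Note_SecretMessage2 is an interactable note actor that shows the second secret message as a full-screen UI.
; Interactwith creates and displays the note widget, switches to UI-only input with a visible cursor, and sets an InNote flag.
; Pressing E while InNote removes the widget and adds a newly created HUD, without restoring input mode or hiding the cursor.
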(event EventBeginPlay
  (Variables|Default|SetbInNote false))

(event EventInteractwith
  (bind _returnvalue (Game|GetPlayerController 0))
  (bind _returnvalue_2 (UserInterface|CreateWidget "/Game/StaticNoise/Blueprints/Actors/notes/SecretMessage/WBP_Note_SecretMessage2UI.WBP_Note_SecretMessage2UI_C"))
  (bind _output_get (Variables|Default|SetNoteUI _returnvalue_2))
  (UserInterface|Viewport|AddtoViewport _output_get 0)
  (Input|SetInputModeUIOnly _returnvalue _output_get "LockInFullscreen" false)
  (Variables|/Script/Engine.PlayerController|SetbShowMouseCursor _returnvalue true)
  (Variables|Default|SetbInNote true))

(event Input|KeyboardEvents|E
  (params (Key :type Key%20Structure :default "None"))
  (:Pressed
    (if (Variables|Default|GetbInNote)
      (Widget|RemovefromParent (stale EventInteractwith _output_get))
      (Variables|Default|SetbInNote false)
      (bind _returnvalue (UserInterface|CreateWidget "/Game/StaticNoise/Blueprints/UI/HUD/HUD.HUD_C" (Game|GetPlayerController 0)))
      (UserInterface|Viewport|AddtoViewport _returnvalue 0))))

(fn ConstructionScript)