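; Office lightbulb actor that acts as an interactable light switch.
; It turns its PointLight on at BeginPlay and tracks the state in a LightOn flag.
; The Interactwith event toggles the light's visibility and that flag, printing a debug message.
; The Lookat event is only a debug stub, with screen and log output both disabled.
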(event EventInteractwith
  (bind _pointlight (Variables|Default|GetPointLight))
  (Development|PrintString "Interacting with light switch")
  (if (Variables|Default|GetbLightOn)
    (Rendering|SetVisibility _pointlight false false)
    (Variables|Default|SetbLightOn false)
    (else
      (Rendering|SetVisibility _pointlight true false)
      (Variables|Default|SetbLightOn true))))

(event EventLookat
  (Development|PrintString "Looking at light switch" false false "(R=0.000000,G=0.660000,B=1.000000,A=1.000000)" 0.01))

(event EventBeginPlay
  (Rendering|SetVisibility (Variables|Default|GetPointLight) true false)
  (Variables|Default|SetbLightOn true))

(fn ConstructionScript)