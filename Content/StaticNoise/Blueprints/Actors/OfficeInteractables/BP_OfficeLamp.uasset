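; BP_OfficeLamp is an interactable office lamp whose point light the player can switch on and off.
; BeginPlay turns the light on, and each Interactwith event toggles the PointLight's visibility, tracking the state in LightOn.
; The Lookat event and construction script are empty.
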(event EventInteractwith
  (bind _pointlight (Variables|Default|GetPointLight))
  (if (Variables|Default|GetbLightOn)
    (Rendering|SetVisibility _pointlight false false)
    (Variables|Default|SetbLightOn false)
    (else
      (Rendering|SetVisibility _pointlight true false)
      (Variables|Default|SetbLightOn true))))

(event EventLookat)

(event EventBeginPlay
  (Rendering|SetVisibility (Variables|Default|GetPointLight) true false)
  (Variables|Default|SetbLightOn true))

(fn ConstructionScript)