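; Interactable in-world computer that the player sits at to read voiced emails, ending in the computer's destruction.
; Overlap shows a prompt and enables input; E or gamepad toggles use via FlipFlop, switching screen, cursor, sounds and player state.
; Clickable components step through email sprites and voice-overs.
; The final email triggers a delayed shutdown, static and explosion sounds, and flags the computer destroyed on the player.
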(event OnClicked(CloseEmail)
  (params (TouchedComponent :type Primitive%20Component%20Object%20Reference) (ButtonPressed :type Key%20Structure :default "None"))
  ;[0.08498 0.4594 0] Close Email
  (Audio|Components|Audio|Play (Variables|Default|GetMouse%20Click) 0.0)
  (Audio|Components|Audio|Stop (Variables|Default|GetPlay%20Intro%20Audio))
  (Rendering|Components|Sprite|SetSprite (Variables|Default|GetScreens) 0)
  (Development|SetHiddeninGame (Variables|Default|GetNext%20Email) true false)
  (Development|SetHiddeninGame (Variables|Default|GetNextEmailText) true false)
  (Class|AudioComponent|SetPaused (Variables|Default|GetComputerRunning) false))

(event OnClicked(NextEmail)
  (params (TouchedComponent :type Primitive%20Component%20Object%20Reference) (ButtonPressed :type Key%20Structure :default "None"))
  ;[0.1648 0.5344 0] Next Email
  (Audio|Components|Audio|Play (Variables|Default|GetMouse%20Click) 0.0)
  (Audio|Components|Audio|Stop (Variables|Default|GetPlay%20Intro%20Audio))
  (Audio|Components|Audio|Play (Variables|Default|GetPlay%202nd%20Page) 0.0)
  (Rendering|Components|Sprite|SetSprite (Variables|Default|GetScreens) 0)
  (Development|SetHiddeninGame (Variables|Default|GetNext%20Email) true false)
  (Development|SetHiddeninGame (Variables|Default|GetFinal%20Email) false false)
  (Variables|Default|SetIs%20Not%20Hidden? true))

(event OnClicked(MinigameClick)
  (params (TouchedComponent :type Primitive%20Component%20Object%20Reference) (ButtonPressed :type Key%20Structure :default "None"))
  ;[0.103 0.5104 0] Set Clicked Minigame To True
  (Audio|Components|Audio|Play (Variables|Default|GetMouse%20Click) 0.0)
  (Class|AudioComponent|SetPaused (Variables|Default|GetComputerRunning) true)
  (Variables|Default|SetHas%20Clicked%20Minigame? true))

(event OnClicked(EmailClick)
  (params (TouchedComponent :type Primitive%20Component%20Object%20Reference) (ButtonPressed :type Key%20Structure :default "None"))
  ;[0.06281 0.4271 0] Start Reading Email
  (Audio|Components|Audio|Play (Variables|Default|GetMouse%20Click) 0.0)
  (Rendering|Components|Sprite|SetSprite (Variables|Default|GetScreens) 0)
  (Audio|Components|Audio|Play (Variables|Default|GetPlay%20Intro%20Audio) 0.0)
  (Development|SetHiddeninGame (Variables|Default|GetNext%20Email) false false)
  (Development|SetHiddeninGame (Variables|Default|GetNextEmailText) false false)
  (Class|AudioComponent|SetPaused (Variables|Default|GetComputerRunning) true))

(event OnClicked(FinalEmail)
  (params (TouchedComponent :type Primitive%20Component%20Object%20Reference) (ButtonPressed :type Key%20Structure :default "None"))
  ;[0.1648 0.5344 0] Next Email
  (if (Variables|Default|GetIs%20Not%20Hidden?)
    (Audio|Components|Audio|Stop (Variables|Default|GetPlay%20Intro%20Audio))
    (Audio|Components|Audio|Stop (Variables|Default|GetPlay%202nd%20Page))
    (Audio|Components|Audio|Play (Variables|Default|GetFinal%20Email%20Voice) 0.0)
    (Rendering|Components|Sprite|SetSprite (Variables|Default|GetScreens) 0)
    (Development|SetHiddeninGame (Variables|Default|GetFinal%20Email) true false)
    ;[0.195 0.5469 0] Destroy Computer
    (Utilities|FlowControl|Delay 0.2 21.0)
    (Utilities|FlowControl|Sequence
      (:then_0
        (bind _asplayer_bp (Utilities|Casting|CastTo (Game|GetPlayerCharacter 0)))
        (Variables|Default|SetIs%20Computer%20Destoryed? _asplayer_bp true)
        (Variables|Default|SetIs%20Using%20Computer? _asplayer_bp false)
        (Widget|RemovefromParent (Variables|Default|GetPress%20E))
        (Variables|/Script/Engine.PlayerController|SetbShowMouseCursor (Game|GetPlayerController 0) false)
        (Audio|Components|Audio|Play (Variables|Default|GetChair%20Sit) 0.0)
        (Audio|Components|Audio|Play (Variables|Default|GetComputerTurnOff) 0.0)
        (Audio|Components|Audio|Stop (Variables|Default|GetChair%20Rocking))
        (Audio|Components|Audio|Stop (Variables|Default|GetComputerRunning))
        (Audio|Components|Audio|Stop (Variables|Default|GetComputerTurnOn))
        (Audio|Components|Audio|Stop (Variables|Default|GetPlay%202nd%20Page))
        (Audio|Components|Audio|Stop (Variables|Default|GetPlay%20Intro%20Audio))
        (Audio|Components|Audio|Stop (Variables|Default|GetFinal%20Email%20Voice))
        (Development|SetHiddeninGame (Variables|Default|GetScreens) true false))
      (:then_1
        (Audio|Components|Audio|Play (Variables|Default|GetComputer%20Static) 0.0)
        (Utilities|FlowControl|Delay 0.2 5.0)
        (Audio|Components|Audio|Play (Variables|Default|GetExplosion) 0.0)))))

(event EventBeginPlay
  ;[0.1113 0.6146 0] Create both WIDG references at the start of the game
  (Utilities|FlowControl|Sequence
    (:then_0
      (bind _returnvalue (UserInterface|CreateWidget 0))
      (Variables|Default|SetPress%20E _returnvalue)
      (Development|SetHiddeninGame (Variables|Default|GetNext%20Email) true false)
      (Development|SetHiddeninGame (Variables|Default|GetNextEmailText) true false))
    (:then_1
      (Variables|/Script/Engine.PlayerController|SetbEnableClickEvents (Game|GetPlayerController 0) true))
    (:then_2
      (Variables|Default|SetHas%20Clicked%20Minigame? false))
    (:then_3
      (Development|SetHiddeninGame (Variables|Default|GetScreens) true false))
    (:then_4
      ;[0.1648 0.5344 0] Next Email
      (Development|SetHiddeninGame (Variables|Default|GetFinal%20Email%20Text) true false)
      (Variables|Default|SetIs%20Not%20Hidden? false))))

(event Collision|EventActorBeginOverlap
  (params (OtherActor :type Actor%20Object%20Reference))
  ;[0.1034 0.4271 0] Show E To Interact Widget
  (Utilities|Casting|CastTo OtherActor)
  (Utilities|FlowControl|Sequence
    (:then_0
      (Input|EnableInput (Game|GetPlayerController 0)))
    (:then_1
      (UserInterface|Viewport|AddtoViewport (Variables|Default|GetPress%20E) 0))))

(event Collision|EventActorEndOverlap
  (params (OtherActor :type Actor%20Object%20Reference))
  ;[0.1265 0.4948 0] Remove Everything
  (Utilities|Casting|CastTo OtherActor)
  (Widget|RemovefromParent (Variables|Default|GetPress%20E))
  (Audio|Components|Audio|Stop (Variables|Default|GetPlay%20Intro%20Audio))
  (Input|DisableInput (Game|GetPlayerController 0))
  (Development|SetHiddeninGame (Variables|Default|GetScreens) true false)
  (Audio|Components|Audio|Stop (Variables|Default|GetChair%20Rocking)))

(event Input|GamepadEvents|GamepadFaceButtonLeft
  (params (Key :type Key%20Structure :default "None"))
  (bind _returnvalue (Game|GetPlayerController 0))
  (bind _computerrunning (Variables|Default|GetComputerRunning))
  (bind _chair_rocking (Variables|Default|GetChair%20Rocking))
  ;[0.07929 0.3958 0] Show Computer
  (:Pressed
    (if (not (Variables|Default|GetIs%20Computer%20Destoryed? (stale _asplayer_bp)))
      (bind _asplayer_bp (Utilities|Casting|CastTo (Game|GetPlayerCharacter 0)))
      (Utilities|FlowControl|FlipFlop
        (:A
          (Variables|Default|SetIs%20Using%20Computer? _asplayer_bp true)
          (Widget|RemovefromParent (Variables|Default|GetPress%20E))
          (Variables|/Script/Engine.PlayerController|SetbShowMouseCursor _returnvalue true)
          (Audio|Components|Audio|Play (Variables|Default|GetChair%20Sit) 0.0)
          (Audio|Components|Audio|Play (Variables|Default|GetComputerTurnOn) 0.0)
          (Utilities|FlowControl|Delay 0.2 1.0)
          (Audio|Components|Audio|Play _computerrunning 0.0)
          (Development|SetHiddeninGame (Variables|Default|GetScreens) false false)
          (Utilities|FlowControl|Delay 0.2 2.0 :!label _label)
          (Audio|Components|Audio|Play _chair_rocking 0.0)
          (Utilities|FlowControl|Delay 0.2 13.0)
          (goto _label))
        (:B
          (Variables|Default|SetIs%20Using%20Computer? _asplayer_bp false)
          (UserInterface|Viewport|AddtoViewport (Variables|Default|GetPress%20E) 0)
          (Variables|/Script/Engine.PlayerController|SetbShowMouseCursor _returnvalue false)
          (Audio|Components|Audio|Play (Variables|Default|GetChair%20Sit) 0.0)
          (Audio|Components|Audio|Play (Variables|Default|GetComputerTurnOff) 0.0)
          (Audio|Components|Audio|Stop _computerrunning)
          (Audio|Components|Audio|Stop _chair_rocking)
          (Audio|Components|Audio|Stop (Variables|Default|GetPlay%202nd%20Page))
          (Audio|Components|Audio|Stop (Variables|Default|GetPlay%20Intro%20Audio))
          (Audio|Components|Audio|Stop (Variables|Default|GetFinal%20Email%20Voice))
          (Development|SetHiddeninGame (Variables|Default|GetScreens) true false))))))

(event Input|KeyboardEvents|E
  (params (Key :type Key%20Structure :default "None"))
  (bind _returnvalue (Game|GetPlayerController 0))
  (bind _computerrunning (Variables|Default|GetComputerRunning))
  (bind _chair_rocking (Variables|Default|GetChair%20Rocking))
  ;[0.07929 0.3958 0] Show Computer
  (:Pressed
    (if (not (Variables|Default|GetIs%20Computer%20Destoryed? (stale _asplayer_bp)))
      (bind _asplayer_bp (Utilities|Casting|CastTo (Game|GetPlayerCharacter 0)))
      (Utilities|FlowControl|FlipFlop
        (:A
          (Variables|Default|SetIs%20Using%20Computer? _asplayer_bp true)
          (Widget|RemovefromParent (Variables|Default|GetPress%20E))
          (Variables|/Script/Engine.PlayerController|SetbShowMouseCursor _returnvalue true)
          (Audio|Components|Audio|Play (Variables|Default|GetChair%20Sit) 0.0)
          (Audio|Components|Audio|Play (Variables|Default|GetComputerTurnOn) 0.0)
          (Utilities|FlowControl|Delay 0.2 1.0)
          (Audio|Components|Audio|Play _computerrunning 0.0)
          (Development|SetHiddeninGame (Variables|Default|GetScreens) false false)
          (Utilities|FlowControl|Delay 0.2 2.0 :!label _label)
          (Audio|Components|Audio|Play _chair_rocking 0.0)
          (Utilities|FlowControl|Delay 0.2 13.0)
          (goto _label))
        (:B
          (Variables|Default|SetIs%20Using%20Computer? _asplayer_bp false)
          (UserInterface|Viewport|AddtoViewport (Variables|Default|GetPress%20E) 0)
          (Variables|/Script/Engine.PlayerController|SetbShowMouseCursor _returnvalue false)
          (Audio|Components|Audio|Play (Variables|Default|GetChair%20Sit) 0.0)
          (Audio|Components|Audio|Play (Variables|Default|GetComputerTurnOff) 0.0)
          (Audio|Components|Audio|Stop _computerrunning)
          (Audio|Components|Audio|Stop _chair_rocking)
          (Audio|Components|Audio|Stop (Variables|Default|GetPlay%202nd%20Page))
          (Audio|Components|Audio|Stop (Variables|Default|GetPlay%20Intro%20Audio))
          (Audio|Components|Audio|Stop (Variables|Default|GetFinal%20Email%20Voice))
          (Development|SetHiddeninGame (Variables|Default|GetScreens) true false))))))

(fn ConstructionScript)