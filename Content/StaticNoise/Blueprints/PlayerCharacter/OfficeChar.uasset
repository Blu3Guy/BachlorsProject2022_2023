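; First-person player character handling movement, look, run, crouch with vignette, zoom, flashlight, pause menu and interaction.
; Looping 0.1-second timers run camera traces that drive cine camera autofocus and detect Interactable actors, toggling a hand HUD and enabling E to interact.
; Timelines animate zoom FOV and crouch capsule height, while Tick sets walk speed and forward-axis input plays idle or run camera shakes by velocity.
; IsCrouched is inverted: pressing crouch sets it false.
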(event Custom|FocusEvent
  (bind _cinecamera (Variables|Default|GetCineCamera))
  (bind _cinecamera_2 (Variables|Default|GetCineCamera))
  (bind _returnvalue (Transformation|GetWorldLocation _cinecamera_2))
  ;[1 1 1] TraceChannel.
  (bind (_outhit _returnvalue_2) (Collision|LineTraceByChannel _returnvalue (+ _returnvalue (* (Math|Vector|GetForwardVector _cinecamera_2) (Math|Conversions|ToVector(Float) 1e+04))) "TraceTypeQuery1" false 0 "None"))
  (if _returnvalue_2
    (Variables|Default|SetfocusDistance (Math|Vector|VectorLength (- (.Location (Collision|BreakHitResult _outhit)) (Transformation|GetWorldLocation (Variables|Default|GetCineCamera)))))
    (Variables|/Script/CinematicCamera.CineCameraComponent|SetFocusSettings _cinecamera (Utilities|Struct|MakeCameraFocusSettings "Manual" (Variables|Default|GetfocusDistance) "(ActorToTrack=None,RelativeOffset=(X=0.000000,Y=0.000000,Z=0.000000))" true))
    (Variables|/Script/CinematicCamera.CineCameraComponent|SetCurrentAperture _cinecamera (Variables|Default|GetFocusScale))
    (else
      (Variables|Default|SetfocusDistance 0.0))))

(event Custom|traceObjectCheck
  (bind _cinecamera (Variables|Default|GetCineCamera))
  (bind _returnvalue (Transformation|GetWorldLocation _cinecamera))
  ;[1 1 1] TraceChannel.
  (bind _outhit (Collision|LineTraceByChannel _returnvalue (+ _returnvalue (* (Math|Vector|GetForwardVector _cinecamera) (Math|Conversions|ToVector(Float) 5e+02))) "TraceTypeQuery1" false 0 "None"))
  (if (Utilities|DoesObjectImplementInterface (.HitActor (Collision|BreakHitResult _outhit)) "/Game/StaticNoise/Blueprints/Interface/Interactable.Interactable_C")
    (Variables|Default|SetbLookingAtObject true)
    (Development|PrintString "Interactable object hit" true false "(R=0.000000,G=0.660000,B=1.000000,A=1.000000)" 0.01)
    (bind _asinteractable (Utilities|Casting|CastToInteractable (.HitActor (Collision|BreakHitResult _outhit)))
      (:then
        (Development|PrintString "Cast sucess " true true "(R=0.000000,G=0.660000,B=1.000000,A=1.000000)" 0.01)
        (Default|Lookat _asinteractable))
      (:CastFailed
        (Development|PrintString "Cast Failed " true true "(R=0.000000,G=0.660000,B=1.000000,A=1.000000)" 0.01)))
    (else
      (Variables|Default|SetbLookingAtObject false))))

(event Custom|objectCheckHand
  (bind _hand (Variables|Default|GetHand))
  (if (Variables|Default|GetbLookingAtObject)
    (UserInterface|Viewport|AddtoViewport _hand 0)
    (else
      (Widget|RemovefromParent _hand))))

(event EventBeginPlay
  (Utilities|FlowControl|Sequence
    (:then_0
      (bind _returnvalue (UserInterface|CreateWidget "/Game/StaticNoise/Blueprints/UI/HUD/HUD_hand.HUD_hand_C"))
      (Variables|Default|SetHand _returnvalue)
      (Variables|Default|SetbIsRunning false)
      (Variables|Default|SetbEKeyIsPressed false)
      (Variables|Default|SetRunSpeed 3.5e+02)
      (Variables|Default|SetDefaultCameraLocation (Variables|/Script/Engine.SceneComponent|GetRelativeLocation (Variables|Default|GetCineCamera))))
    (:then_1
      (Utilities|Time|SetTimerbyFunctionName 0 "FocusEvent" 0.1 true))
    (:then_2
      (Utilities|Time|SetTimerbyFunctionName 0 "traceObjectCheck" 0.1 true))
    (:then_3
      (Utilities|Time|SetTimerbyFunctionName 0 "objectCheckHand" 0.1 true))))

(event EventTick
  (params (DeltaSeconds :type Float%20%28single-precision%29))
  (bind _charactermovement (Variables|Character|GetCharacterMovement))
  (bind _charactermovement_2 (Variables|Character|GetCharacterMovement))
  (if (Variables|Default|GetIsCrouched)
    (Variables|/Script/Engine.CharacterMovementComponent|SetMaxWalkSpeed _charactermovement_2 (Variables|Default|GetWalkSpeed))
    (else
      (Variables|/Script/Engine.CharacterMovementComponent|SetMaxWalkSpeed _charactermovement_2 (Variables|Default|GetCrouchSpeed))))
  (if (Variables|Default|GetbIsRunning)
    (if (Variables|Default|GetIsCrouched)
      (Variables|/Script/Engine.CharacterMovementComponent|SetMaxWalkSpeed _charactermovement (Variables|Default|GetRunSpeed)))
    (else
      (Variables|/Script/Engine.CharacterMovementComponent|SetMaxWalkSpeed _charactermovement (Variables|Default|GetWalkSpeed)))))

(event Input|ActionEvents|InputActionPause
  (params (Key :type Key%20Structure :default "None"))
  (bind _returnvalue (Game|GetPlayerController 0))
  (:Pressed
    ;[1 1 1] Pause/Un-pause Game
    (Utilities|IsValid (Variables|Default|GetPause%20Menu%20REF)
      (:Is%20Valid
        _)
      (:Is%20Not%20Valid
        (bind _returnvalue_2 (UserInterface|CreateWidget "/Game/StaticNoise/Blueprints/UI/Pause_Menu/Pause_Menu.Pause_Menu_C"))
        (Variables|Default|SetPause%20Menu%20REF _returnvalue_2)))
    (if (Game|IsGamePaused)
      (Widget|RemovefromParent (Variables|Default|GetPause%20Menu%20REF))
      (Game|SetGamePaused false)
      (Variables|/Script/Engine.PlayerController|SetbShowMouseCursor _returnvalue false)
      (Input|SetInputModeGameOnly _returnvalue false)
      (else
        (UserInterface|Viewport|AddtoViewport (Variables|Default|GetPause%20Menu%20REF) 0)
        (Game|SetGamePaused true)
        (Variables|/Script/Engine.PlayerController|SetbShowMouseCursor _returnvalue true)
        (Input|SetInputModeUIOnly _returnvalue (Variables|Default|GetPause%20Menu%20REF) "LockInFullscreen" false)))))

(event Input|ActionEvents|InputActionFlashlight
  (params (Key :type Key%20Structure :default "None"))
  ;[1 1 1] Flashlight
  (:Pressed
    (Rendering|SetVisibility (Variables|Default|GetFlashlight) (not (Rendering|IsVisible (Variables|Default|GetFlashlight))) false)))

(event Input|AxisEvents|InputAxisForwards/Backwards
  (params (AxisValue :type Float%20%28single-precision%29))
  (bind _returnvalue (Transformation|GetVelocity))
  (bind _returnvalue_2 (Transformation|GetActorLocation))
  (bind _returnvalue_3 (Math|Vector|VectorLength _returnvalue))
  ;[1 1 1] Basic Movement
  (Pawn|Input|AddMovementInput (Math|Vector|GetForwardVector (Math|Rotator|MakeRotator 0.0 0.0 (.Yaw (Math|Rotator|BreakRotator (Pawn|GetControlRotation :!class /Script/Engine.Pawn))))) AxisValue false)
  ;[1 1 1] Camera Shake
  (if (<= _returnvalue_3 1.0)
    (Camera|PlayWorldCameraShake "/Game/StaticNoise/Blueprints/PlayerCharacter/IdleShake.IdleShake_C" _returnvalue_2 1e+02 0.0)
    (elif (>= _returnvalue_3 349.0)
      (Camera|PlayWorldCameraShake "/Game/StaticNoise/Blueprints/PlayerCharacter/RunShake.RunShake_C" _returnvalue_2 1e+02 0.0))))

(event Input|AxisEvents|InputAxisRight/Left
  (params (AxisValue :type Float%20%28single-precision%29))
  ;[1 1 1] Basic Movement
  (Pawn|Input|AddMovementInput (Math|Vector|GetRightVector (Math|Rotator|MakeRotator 0.0 0.0 (.Yaw (Math|Rotator|BreakRotator (Pawn|GetControlRotation :!class /Script/Engine.Pawn))))) AxisValue false))

(event Input|AxisEvents|InputAxisViewUpDown
  (params (AxisValue :type Float%20%28single-precision%29))
  ;[1 1 1] Basic Camera Movement
  (Pawn|Input|AddControllerPitchInput (* AxisValue (Variables|Default|GetMouseSensitivity_0) (Utilities|Time|GetWorldDeltaSeconds))))

(event Input|AxisEvents|InputAxisviewLeftRight
  (params (AxisValue :type Float%20%28single-precision%29))
  ;[1 1 1] Basic Camera Movement
  (Pawn|Input|AddControllerYawInput (* AxisValue (Variables|Default|GetMouseSensitivity_0) (Utilities|Time|GetWorldDeltaSeconds))))

(event Input|KeyboardEvents|LeftShift
  (params (Key :type Key%20Structure :default "None"))
  (:Pressed
    (Variables|Default|SetbIsRunning true))
  (:Released
    (Variables|Default|SetbIsRunning false)))

(event Input|KeyboardEvents|LeftCtrl
  (params (Key :type Key%20Structure :default "None"))
  ;[1 1 1] Crouch
  (:Pressed
    (Variables|Default|SetIsCrouched false)
    (bind (_direction _offsetvalue _vinette) (Timeline|Crouch%20Height PlayFromStart)
      (:Update
        (Components|Capsule|SetCapsuleHalfHeight (Variables|Collision|GetCapsuleComponent) (- 96.0 (* _offsetvalue (Variables|Default|GetHalfHeightOffset))) true)
        (Variables|/Script/Engine.CameraComponent|SetPostProcessSettings (Variables|Default|GetCineCamera) (Utilities|Struct|MakePostProcessSettings _vinette)))))
  (:Released
    (Variables|Default|SetIsCrouched true)
    (Timeline|Crouch%20Height ReverseFromEnd)))

(event Input|KeyboardEvents|E
  (params (Key :type Key%20Structure :default "None"))
  (:Pressed
    (if (Variables|Default|GetbLookingAtObject)
      (Default|Interactwith (stale Custom|traceObjectCheck _asinteractable)))))

(event Input|MouseEvents|RightMouseButton
  (params (Key :type Key%20Structure :default "None"))
  ;[1 1 1] zoom
  (:Pressed
    (bind _zoom (Timeline|Zoom Play)
      (:Update
        (Camera|SetFieldOfView (Variables|Default|GetCineCamera) _zoom))))
  (:Released
    (Timeline|Zoom Reverse)))

(fn ConstructionScript)